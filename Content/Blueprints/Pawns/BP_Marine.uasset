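; Player marine pawn for a twin-stick style shooter, with world-axis movement, a HUD, health and a kill counter.
; Aim sets control rotation from thumbstick angle or smoothed mouse-velocity direction, both deadzoned, switching on the last key pressed.
; Firing runs a looping timer of muzzle-socket line traces that apply damage and impact effects, alongside muzzle flash and looped audio.
; Zero health sets Dead, which stops firing and blocks movement, aim and further damage.
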(event EventBeginPlay
  ;[1 0.09903 0.2591] Create HUD
  (bind _returnvalue (UserInterface|CreateWidget "/Game/UI/W_PlayerHUD.W_PlayerHUD_C" 0 self))
  (UserInterface|Viewport|AddtoViewport _returnvalue 0))

(event EventTick
  (params (DeltaSeconds :type Float%20%28single-precision%29))
  ;[0.3896 0.4575 1] Update Aim Each Frame
  (GameInput|UpdatePlayerAim))

(event Game|Damage|EventAnyDamage
  (params (Damage :type Float%20%28single-precision%29) (DamageType :type Damage%20Type%20Object%20Reference) (InstigatedBy :type Controller%20Object%20Reference) (DamageCauser :type Actor%20Object%20Reference))
  ;[0.6445 0.1096 1] Player Damage
  (if (PlayerFunctions|IsAlive)
    (bind _health (PlayerFunctions|DecreaseHealth Damage))
    (if (== _health 0.0)
      (Variables|PlayerProperties|SetDead true)
      (if (Variables|PlayerProperties|GetIs%20Firing)
        (WeaponFunctions|StopFiringWeapon)))))

(event Input|ActionEvents|InputActionFireWeapon
  (params (Key :type Key%20Structure :default "None"))
  ;[0.4557 1 0.2946] Weapon Firing
  (:Pressed
    (WeaponFunctions|StartFiringWeapon))
  (:Released
    (WeaponFunctions|StopFiringWeapon)))

(event Input|AxisEvents|InputAxisMoveRight/Left
  (params (AxisValue :type Float%20%28single-precision%29))
  ;[1 0.999 0.08523] Player Movement
  (if (PlayerFunctions|IsAlive)
    (Pawn|Input|AddMovementInput "0,1.000000,0.000000" AxisValue false)))

(event Input|AxisEvents|InputAxisMoveForwards/Backwards
  (params (AxisValue :type Float%20%28single-precision%29))
  ;[1 0.999 0.08523] Player Movement
  (if (PlayerFunctions|IsAlive)
    (Pawn|Input|AddMovementInput "1.000000,0.000000,0.0" AxisValue false)))

(event Input|KeyboardEvents|AnyKey
  (params (Key :type Key%20Structure :default "None"))
  ;[1 0.5861 0.08121] Controller Active Check
  (:Pressed
    (GameInput|CheckifGamepadActive Key)))

(fn ConstructionScript)

(fn UpdatePlayerAim
  (if (PlayerFunctions|IsAlive)
    (if (Variables|GameInputProperties|GetGamepadActive)
      (ThumbstickInput|UpdateThumbstickAim)
      (else
        (MouseInput|UpdateMouseAim)))))

(fn IsThumbstickAboveDeadzone
  (return (> (ThumbstickInput|GetThumbstickDeflectionAmount) (Variables|ThumbstickInput|GetThumbstickDeadzone))))

(fn GetThumbstickAimDirection
  (return (Math|Rotator|MakeRotator 0.0 0.0 (Class|KismetMathLibrary|DegAtan2 (Input|AxisValues|GetThumbstickAimRight/Left) (Input|AxisValues|GetThumbstickAimUp/Down)))))

(fn GetMouseVelocity
  (bind _returnvalue (Game|GetPlayerController 0))
  (bind (_deltax _deltay) (Class|PlayerController|GetInputMouseDelta _returnvalue))
  (return (/ (Math|Vector2D|MakeVector2D _deltax _deltay) (Utilities|Time|GetWorldDeltaSeconds))))

(fn GetThumbstickDeflectionAmount
  (return (Math|Vector2D|Vector2DLength (Math|Vector2D|MakeVector2D (Input|AxisValues|GetThumbstickAimRight/Left) (Input|AxisValues|GetThumbstickAimUp/Down)))))

(fn IsMouseAboveDeadzone
  (return (> (Math|Vector2D|Vector2DLength (MouseInput|GetMouseVelocity)) (Variables|MouseInput|GetMouseDeadzone))))

(fn GetRotationfromMouse
  (bind _returnvalue (MouseInput|GetMouseVelocity))
  (return (Math|Rotator|MakeRotator 0.0 0.0 (Class|KismetMathLibrary|DegAtan2 (.x _returnvalue) (.y _returnvalue)))))

(fn UpdateMouseAim
  (if (MouseInput|IsMouseAboveDeadzone)
    (Pawn|SetControlRotation (Game|GetPlayerController 0) (MouseInput|GetMouseAimDirection))))

(fn UpdateThumbstickAim
  (if (ThumbstickInput|IsThumbstickAboveDeadzone)
    (Pawn|SetControlRotation (Game|GetPlayerController 0) (ThumbstickInput|GetThumbstickAimDirection))))

(fn GetMouseAimDirection
  (return (Math|Interpolation|RInterpTo (Pawn|GetControlRotation (Game|GetPlayerController 0) :!class /Script/Engine.Controller) (MouseInput|GetRotationfromMouse) (Utilities|Time|GetWorldDeltaSeconds) (Variables|MouseInput|GetMouse%20Smoothing%20Strength))))

(fn CheckifGamepadActive
  (params (Key :type Key%20Structure%20%28by%20ref%29))
  (Variables|GameInputProperties|SetGamepadActive (Class|KismetInputLibrary|KeyIsGamepadKey Key)))

(fn StartFiringWeapon
  (if (PlayerFunctions|IsAlive)
    (Components|Activation|Activate (Variables|Default|GetP_AssaultRifle_MF) false)
    (bind _returnvalue (Audio|SpawnSound2D "/Game/Sounds/Weapon_AssaultRifle/Stereo/RifleSoundLoop_Cue.RifleSoundLoop_Cue" 1.0 1.0 0.0 0))
    (Variables|Default|SetWeapon%20Fire%20Sound _returnvalue)
    (Variables|PlayerProperties|SetIs%20Firing true)
    (WeaponFunctions|WeaponTrace)
    (Utilities|Time|SetTimerbyFunctionName 0 "Weapon Trace" (Variables|WeaponProperties|GetWeapon%20Fire%20Rate) true)))

(fn StopFiringWeapon
  (bind _weapon_fire_sound (Variables|Default|GetWeapon%20Fire%20Sound))
  (Components|Activation|Deactivate (Variables|Default|GetP_AssaultRifle_MF))
  (Utilities|IsValid _weapon_fire_sound
    (:Is%20Valid
      (Audio|Components|Audio|Stop _weapon_fire_sound)
      (Utilities|Time|ClearTimerbyFunctionName 0 "Weapon Trace")
      (Audio|SpawnSound2D "/Game/Sounds/Weapon_AssaultRifle/Stereo/RifleFireEnd_Cue.RifleFireEnd_Cue" 1.0 1.0 0.0 0)
      (Variables|PlayerProperties|SetIs%20Firing false))))

(fn DecreaseHealth
  (params (Damage%20Amount :type Float%20%28single-precision%29))
  (bind _output_get (Variables|PlayerProperties|SetPlayer%20Health (Math|Float|Clamp(Float) (- (Variables|PlayerProperties|GetPlayer%20Health) Damage%20Amount) 0.0 (Variables|PlayerProperties|GetMax%20Health))))
  (return _output_get))

(fn IsAlive
  (return (not (Variables|PlayerProperties|GetDead))))

(fn WeaponTrace
  (bind _outhit (Collision|LineTraceByChannel (WeaponFunctions|GetWeaponTraceStartLocation) (WeaponFunctions|GetWeaponTraceEndLocation) "TraceTypeQuery1" false 0 "None"))
  (if (.bBlockingHit (Collision|BreakHitResult _outhit))
    (WeaponFunctions|SpawnImpactHit (.Location (Collision|BreakHitResult _outhit)))
    (Game|Damage|ApplyDamage (.HitActor (Collision|BreakHitResult _outhit)) (Variables|WeaponProperties|GetDamage%20Per%20Hit) 0 0)))

(fn GetWeaponTraceStartLocation
  (return (Transformation|GetSocketLocation (Variables|Default|GetP_AssaultRifle_MF) "MuzzleFlashSocket")))

(fn GetWeaponTraceEndLocation
  (return (+ (WeaponFunctions|GetWeaponTraceStartLocation) (* (Math|Vector|GetForwardVector (Pawn|GetControlRotation :!class /Script/Engine.Pawn)) (Variables|WeaponProperties|GetWeapon%20Range)))))

(fn IncreaseKills
  (Math|Integer|IncrementInt (Variables|PlayerProperties|GetNumber%20of%20Kills)))

(fn SpawnImpactHit
  (params (Hit%20Location :type Vector))
  (Effects|SpawnEmitteratLocation "/Game/Effects/Weapons/Impacts/P_AssaultRifle_IH.P_AssaultRifle_IH" Hit%20Location))

(fn AddHealth
  (params (Health%20to%20Add :type Float%20%28single-precision%29))
  (Variables|PlayerProperties|SetPlayer%20Health (Math|Float|Clamp(Float) (+ (Variables|PlayerProperties|GetPlayer%20Health) Health%20to%20Add) 0.0 (Variables|PlayerProperties|GetMax%20Health))))

(fn IsHealthFull
  (return (== (Variables|PlayerProperties|GetPlayer%20Health) (Variables|PlayerProperties|GetMax%20Health))))