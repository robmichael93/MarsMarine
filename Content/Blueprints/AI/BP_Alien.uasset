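; BP_Alien is an enemy alien that chases the player, attacks in melee and takes damage until killed.
; A looping AIMoveTo drives pursuit, while Tick checks range and plays a swipe montage, pausing movement until it completes.
; DamagePlayer applies hit damage but is not called within this Blueprint.
; At zero health it disables movement and collision, reports the kill to BP_Marine and the game mode, then destroys itself after a delay.
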(event EventBeginPlay
  ;[1 0.5636 0.1369] Pursue Player
  (if (CallFunction|IsAlive) :!label _label
    (AI|AIMoveTo self "0, 0, 0" (Game|Player|GetPlayerPawn 0) 5.0 false
      (:OnSuccess
        _)
      (:OnFail
        _))
    (Utilities|FlowControl|Delay 0.2)
    (goto _label)))

(event EventTick
  (params (DeltaSeconds :type Float%20%28single-precision%29))
  ;[1 0.08327 0.09322] Attack Animations
  (Utilities|CanAttack
    (:Yes
      (MovementFunctions|DeactivateAIMovement)
      (Animation|Montage|PlayMontage (Variables|Character|GetMesh) "/Game/Characters/Enemy_Great_Spider/Animations/SpiderAttackSwipe.SpiderAttackSwipe"
        (:OnCompleted
          (MovementFunctions|ActivateAIMovement))))))

(event Game|Damage|EventAnyDamage
  (params (Damage :type Float%20%28single-precision%29) (DamageType :type Damage%20Type%20Object%20Reference) (InstigatedBy :type Controller%20Object%20Reference) (DamageCauser :type Actor%20Object%20Reference))
  ;[0.1073 1 0.1677] Alien Damage and Death
  (if (CallFunction|IsAlive)
    (bind _health (DamageFunctions|DecreaseHealth Damage))
    (if (== _health 0.0)
      (DamageFunctions|KillAI)
      (Utilities|FlowControl|Delay 3.0)
      (Actor|DestroyActor))))

(fn ConstructionScript)

(fn IsWithinAttackRange
  (return (<= (Transformation|GetDistanceTo (Game|Player|GetPlayerPawn 0)) (Variables|Default|GetAttack%20Range))))

(fn IsAttacking
  (return (Animation|Montage|MontageIsPlaying (Components|SkeletalMesh|GetAnimInstance (Variables|Character|GetMesh)) "/Game/Characters/Enemy_Great_Spider/Animations/SpiderAttackSwipe.SpiderAttackSwipe")))

(fn DeactivateAIMovement
  (bind _charactermovement (Variables|Character|GetCharacterMovement))
  (Components|Movement|StopMovementImmediately _charactermovement)
  (Components|Activation|Deactivate _charactermovement))

(fn ActivateAIMovement
  (Components|Activation|Activate (Variables|Character|GetCharacterMovement) false))

(fn DamagePlayer
  (if (CallFunction|IsAlive)
    (Game|Damage|ApplyDamage (Game|GetPlayerCharacter 0) (Variables|Default|GetDamage%20Per%20Hit) 0 0)))

(fn DecreaseHealth
  (params (Damage%20Amount :type Float%20%28single-precision%29))
  (bind _output_get (Variables|Default|SetHealth (Math|Float|Clamp(Float) (- (Variables|Default|GetHealth) Damage%20Amount) 0.0 (Variables|Default|GetMax%20Health))))
  (return _output_get))

(fn KillAI
  (Variables|Default|SetDead true)
  (MovementFunctions|DeactivateAIMovement)
  (Collision|SetActorEnableCollision false)
  (bind _asbp_marine (Utilities|Casting|CastToBP_Marine (Game|GetPlayerCharacter 0)))
  (Default|IncreaseKills _asbp_marine)
  (bind _asbp_mars_marine_game_mode (Utilities|Casting|CastToBP_MarsMarineGameMode (Game|GetGameMode)))
  (Default|RegisterAlienDeath _asbp_mars_marine_game_mode self))

(fn IsAlive
  (return (not (Variables|Default|GetDead))))